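; Player controller for a pinball game that maps input to flippers, the plunger and table tilt.
; On BeginPlay it finds all flipper actors, sorting them into left and right arrays by type, and takes the first plunger found.
; Flipper and charge inputs call up/down and charge/release on those actors.
; Tilt gives every ball a sideways velocity impulse and plays a camera shake, rolled 180 degrees for the opposite direction.
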(event `self.ReceiveBeginPlay`
  (`self.FindAllplunger`)
  (`self.FindAllFlipers`))

(event `InputAction|left_fliper`
  (params (Key :type "Key Structure"))
  (bind _leftfliper (`self.leftFliper`))
  (:`Pressed`
    (for _array_element _leftfliper
      (`/Game/blueprints/BP_fliper.fliperup` _array_element)))
  (:`Released`
    (for _array_element_2 _leftfliper
      (`/Game/blueprints/BP_fliper.fliperdown` _array_element_2))))

(event `InputAction|right_fliper`
  (params (Key :type "Key Structure"))
  (bind _rightfliper (`self.rightFliper`))
  (:`Pressed`
    (for _array_element _rightfliper
      (`/Game/blueprints/BP_fliper.fliperup` _array_element)))
  (:`Released`
    (for _array_element_2 _rightfliper
      (`/Game/blueprints/BP_fliper.fliperdown` _array_element_2))))

(event `InputAction|charge`
  (params (Key :type "Key Structure"))
  (bind _plunger (`self.plunger`))
  (:`Pressed`
    (`/Game/blueprints/BP_plunger.charge` _plunger))
  (:`Released`
    (`/Game/blueprints/BP_plunger.release` _plunger)))

(event `FindAllFlipers`
  (bind _outactors (`GameplayStatics.GetAllActorsOfClass` "/Game/blueprints/BP_fliper.BP_fliper_C"))
  (for _array_element _outactors
    (switch `/Game/blueprints/E_direction` (`/Game/blueprints/BP_fliper.flipertype` _array_element)
      (:`NewEnumerator0`
        (`KismetArrayLibrary.Array_Add` (`self.leftFliper`) _array_element))
      (:`NewEnumerator1`
        (`KismetArrayLibrary.Array_Add` (`self.rightFliper`) _array_element)))))

(event `FindAllplunger`
  (bind _outactors (`GameplayStatics.GetAllActorsOfClass` "/Game/blueprints/BP_plunger.BP_plunger_C"))
  (set `self.plunger` (`|GetArrayItem` _outactors)))

(event `InputAction|tilt_left`
  (params (Key :type "Key Structure"))
  (:`Pressed`
    (`self.tilt` "NewEnumerator0")))

(event `InputAction|tilt_right`
  (params (Key :type "Key Structure"))
  (:`Pressed`
    (`self.tilt` "NewEnumerator1")))

(fn `tilt`
  (params (direction :type "/Game/blueprints/E_direction Enum" :default "NewEnumerator0"))
  (bind _returnvalue (`PlayerCameraManager.GetCameraRotation` (`GameplayStatics.GetPlayerCameraManager` 0)))
  (bind _outactors (`GameplayStatics.GetAllActorsOfClass` "/Game/blueprints/BP_ball.BP_ball_C"))
  (if (>= (`KismetArrayLibrary.Array_Length` _outactors) 1)
    (for _array_element _outactors
      (`PrimitiveComponent.AddImpulse` (`/Game/blueprints/BP_ball.ball` _array_element) (select `/Game/blueprints/E_direction` direction :`NewEnumerator0` (0.0 -500.0 0.0) :`NewEnumerator1` (0.0 500.0 0.0) :!type "Vector Structure") "None" true))
    (`self.ClientStartCameraShake` "/Game/blueprints/BP_camera_shake.BP_camera_shake_C" 1.0 "UserDefined" (select `/Game/blueprints/E_direction` direction :`NewEnumerator0` _returnvalue :`NewEnumerator1` (`KismetMathLibrary.ComposeRotators` _returnvalue (struct :`Yaw` 180.0))))))

(fn `UserConstructionScript`)
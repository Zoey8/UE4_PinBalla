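; BP_ball is a physics ball that drives itself along world X while being pulled toward the surface beneath it.
; Each Tick adds a velocity-change impulse to the Ball component, scaled by Speed and delta time.
; A downward Visibility line trace from the actor's location supplies the impact normal, and a second impulse against that normal, scaled by Stickness, pushes the ball onto the surface.
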(event `self.ReceiveTick`
  (params (DeltaSeconds :type "Float (single-precision)"))
  (bind _returnvalue (`self.K2_GetActorLocation`))
  (`PrimitiveComponent.AddImpulse` (`self.ball`) (`KismetMathLibrary.MakeVector` (* DeltaSeconds (`self.speed`))) "None" true)
  (bind _outhit (`KismetSystemLibrary.LineTraceSingle` _returnvalue (- _returnvalue (0.0 0.0 500.0)) "TraceTypeQuery1"))
  (`PrimitiveComponent.AddImpulse` (`self.ball`) (* (* (* (`.ImpactNormal` (`GameplayStatics.BreakHitResult` _outhit)) -1) (`self.stickness`)) DeltaSeconds) "None" true))

(fn `UserConstructionScript`)
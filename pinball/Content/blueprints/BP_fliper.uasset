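; BP_fliper is a pinball flipper actor configurable as a left or right flipper through Flipertype.
; The construction script picks start and end rotations for that side, applies the start rotation, and mirrors right flippers with a negative X scale.
; The fliperup event plays a side-specific attached sound and uses MoveComponentTo to snap the flipper to its end rotation.
; The fliperdown event returns it more slowly to the start rotation.
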(event `self.ReceiveBeginPlay`)

(event `fliperup`
  (`GameplayStatics.SpawnSoundAttached` (select `/Game/blueprints/E_direction` (`self.flipertype`) :`NewEnumerator0` "/Game/Assests/sounds/Pinball_FlipperLeft_Cue.Pinball_FlipperLeft_Cue" :`NewEnumerator1` "/Game/Assests/sounds/Pinball_FlipperRight_Cue.Pinball_FlipperRight_Cue" :!type "SoundBase Object Reference") (`self.fliper`) "None" (0.0 0.0 0.0) (struct) "KeepRelativeOffset" false 1.0 1.0 0.0 null null)
  (`KismetSystemLibrary.MoveComponentTo` (`self.fliper`) (`self.K2_GetActorLocation`) (`self.endrotation`) false false 0.03))

(event `fliperdown`
  (`KismetSystemLibrary.MoveComponentTo` (`self.fliper`) (`self.K2_GetActorLocation`) (`self.startrotation`) false false 0.1))

(fn `UserConstructionScript`
  (set `self.startrotation` (select `/Game/blueprints/E_direction` (`self.flipertype`) :`NewEnumerator0` (struct :`Yaw` -70.0) :`NewEnumerator1` (struct :`Yaw` -110.0) :!type "Rotator Structure"))
  (set `self.endrotation` (select `/Game/blueprints/E_direction` (`self.flipertype`) :`NewEnumerator0` (struct :`Yaw` -120.0) :`NewEnumerator1` (struct :`Yaw` -60.0) :!type "Rotator Structure"))
  (`SceneComponent.K2_SetRelativeRotation` (`self.fliper`) (`self.startrotation`) false false)
  (switch `/Game/blueprints/E_direction` (`self.flipertype`)
    (:`NewEnumerator1`
      (`SceneComponent.SetRelativeScale3D` (`self.fliper`) (-1.0 1.0 1.0)))))
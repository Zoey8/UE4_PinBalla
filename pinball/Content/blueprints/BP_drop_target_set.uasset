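; Drop target bank that spells a word across a row of BP_drop_target actors and resets once all have been dropped.
; The construction script uppercases Poststring and spawns one lettered child actor per character, evenly spaced by the distance between Post1 and Post2.
; It binds to each target's drop event to count down TargetCounter.
; At zero, TargetDropProcess waits briefly, resets every target and restores the count.
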(event `TargetDropProcess`
  (bind _droptargets (`self.DropTargets`))
  (bind _result (`/Engine/EditorBlueprintResources/StandardMacros.DecrementInt` (`self.targetCounter`))
    (:`  `
      (if (<= _result 0)
        (`KismetSystemLibrary.Delay` 1.0)
        (for _array_element _droptargets
          (`/Game/blueprints/BP_drop_target.reset_drop` _array_element)
          (set `self.targetCounter` (`KismetArrayLibrary.Array_Length` _droptargets)))))))

(fn `UserConstructionScript`
  (bind _post1 (`self.post1`))
  (`parent.UserConstructionScript`)
  (bind _output_get (set `self.poststring` (`KismetTextLibrary.TextToUpper` (`self.poststring`))))
  (bind _returnvalue (`KismetStringLibrary.GetCharacterArrayFromString` (`KismetTextLibrary.Conv_TextToString` _output_get)))
  (bind _returnvalue_2 (`KismetArrayLibrary.Array_Length` _returnvalue))
  (set `self.targetCounter` _returnvalue_2)
  (for (_array_element _array_index) _returnvalue
    (bind _returnvalue_3 (`AddComponent|NODE_AddChildActorComponent-0` :`RelativeTransform` (`KismetMathLibrary.MakeTransform` (+ (* (`SceneComponent.GetForwardVector` _post1) (* (+ _array_index 1) (/ (`KismetMathLibrary.VSize` (- (`SceneComponent.RelativeLocation` (`self.post1`)) (`SceneComponent.RelativeLocation` (`self.post2`)))) (`KismetMathLibrary.Conv_IntToDouble` (+ _returnvalue_2 1))))) (* (`SceneComponent.GetRightVector` _post1) 30)) (`SceneComponent.K2_GetComponentRotation` _post1))))
    (bind _asbp_drop_target (cast `/Game/blueprints/BP_drop_target` (`ChildActorComponent.ChildActor` _returnvalue_3)))
    (`KismetArrayLibrary.Array_Add` (`self.DropTargets`) _asbp_drop_target)
    (`TextRenderComponent.K2_SetText` (`/Game/blueprints/BP_drop_target.drop_text` _asbp_drop_target) (`KismetTextLibrary.Conv_StringToText` _array_element))
    (add `/Game/blueprints/BP_drop_target.OnTargetDrop` _asbp_drop_target (`|CreateDelegate` :!event `TargetDropProcess`))))
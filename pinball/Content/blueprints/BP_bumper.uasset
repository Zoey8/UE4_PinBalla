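; BP_bumper is a pinball-style bumper that knocks any overlapping BP_ball away from its center.
; On overlap it replaces the ball's physics velocity with a fixed-speed vector pointing outward from the bumper's location.
; Each hit also plays an attached sound, spawns a particle effect, and restarts a timeline that moves the BumperBot part vertically and drives the bumper material's emissive glow.
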(event `self.ReceiveActorBeginOverlap`
  (params (OtherActor :type "Actor Object Reference"))
  (bind _asbp_ball (cast `/Game/blueprints/BP_ball` OtherActor))
  (`self.bump` _asbp_ball))

(event `bump`
  (params (ball :type "/Game/blueprints/BP_ball Object Reference"))
  (`PrimitiveComponent.SetPhysicsLinearVelocity` (`/Game/blueprints/BP_ball.ball` ball) (* (`KismetMathLibrary.GetDirectionUnitVector` (`self.K2_GetActorLocation`) (`self.K2_GetActorLocation` ball)) 3000.0) false "None")
  (`GameplayStatics.SpawnSoundAttached` "/Game/Assests/sounds/bumper.bumper" (`self.bumper`) "None" (0.0 0.0 0.0) (struct) "KeepRelativeOffset" false 1.0 1.0 0.0 null null)
  (`GameplayStatics.SpawnEmitterAtLocation` "/Game/Assests/particles/P_bumper.P_bumper" (`SceneComponent.K2_GetComponentLocation` (`self.bumper`)))
  (bind (_direction _bumpera) (`Timeline|BumperTimeLine` :!via `PlayFromStart`)
    (:`Update`
      (`SceneComponent.K2_SetRelativeLocation` (`self.bumperBot`) (`KismetMathLibrary.VLerp` (0.0 0.0 0.0) (0.0 0.0 -70.0) _bumpera) false false)
      (`MeshComponent.SetScalarParameterValueOnMaterials` (`self.bumper`) "emissive" (`KismetMathLibrary.Lerp` 0.0 20.0 _bumpera)))))

(fn `UserConstructionScript`)